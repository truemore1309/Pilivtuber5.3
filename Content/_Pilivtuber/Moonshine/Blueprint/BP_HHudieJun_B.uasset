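; MetaHuman-style character Blueprint with ARKit Live Link facial capture and keyboard-toggled expressions.
; On BeginPlay it copies eyelash opacity to the lower-LOD material when hair strands are disabled, starts looping slot montages on Head and Body, and passes Live Link settings to the Head's ARKit AnimInstance.
; Keys 1–6 each use a FlipFlop to play or reverse a Timeline that blends an emotion morph target on the Head.
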(event `self.ReceiveBeginPlay`
  (bind _head (`self.Head`))
  (bind _returnvalue (`KismetSystemLibrary.GetConsoleVariableIntValue` "r.HairStrands.Strands"))
  (if (not (`KismetMathLibrary.Conv_IntToBool` _returnvalue))
    (bind _asmaterial_instance_dynamic (cast `MaterialInstanceDynamic` (`PrimitiveComponent.GetMaterial` _head 10)))
    (bind _asmaterial_instance_dynamic_2 (cast `MaterialInstanceDynamic` (`PrimitiveComponent.GetMaterial` _head 6)))
    (bind _returnvalue_2 (`MaterialInstanceDynamic.K2_GetScalarParameterValue` _asmaterial_instance_dynamic "Opacity"))
    (`MaterialInstanceDynamic.SetScalarParameterValue` _asmaterial_instance_dynamic_2 "Opacity" _returnvalue_2)
    (bind _returnvalue_3 (`MaterialInstanceDynamic.K2_GetScalarParameterValue` _asmaterial_instance_dynamic "OpacityRT"))
    (`MaterialInstanceDynamic.SetScalarParameterValue` _asmaterial_instance_dynamic_2 "OpacityRT" _returnvalue_3))
  (`AnimInstance.PlaySlotAnimationAsDynamicMontage` (`SkeletalMeshComponent.GetAnimInstance` (`self.Head`)) null "DefaultSlot" 0.25 0.25 1.0 10000 -1.0 0.0)
  (`self.ARKit_Setup`)
  (`AnimInstance.PlaySlotAnimationAsDynamicMontage` (`SkeletalMeshComponent.GetAnimInstance` (`self.Body`)) null "DefaultSlot" 0.25 0.25 1.0 10000 -1.0 0.0))

(event `Key|One`
  (params (Key :type "Key Structure"))
  (:`Pressed`
    (`/Engine/EditorBlueprintResources/StandardMacros.FlipFlop`
      (:`A`
        (bind (_direction _frightened) (`Timeline|Timeline_1` :!label _label)
          (:`Update`
            (`SkeletalMeshComponent.SetMorphTarget` (`self.Head`) "frightened" _frightened true))))
      (:`B`
        (goto _label :!via `ReverseFromEnd`)))))

(event `Key|Two`
  (params (Key :type "Key Structure"))
  (:`Pressed`
    (`/Engine/EditorBlueprintResources/StandardMacros.FlipFlop`
      (:`A`
        (bind (_direction _frightened) (`Timeline|Timeline_4` :!label _label_2)
          (:`Update`
            (`SkeletalMeshComponent.SetMorphTarget` (`self.Head`) "surprised" _frightened true))))
      (:`B`
        (goto _label_2 :!via `ReverseFromEnd`)))))

(event `Key|Three`
  (params (Key :type "Key Structure"))
  (:`Pressed`
    (`/Engine/EditorBlueprintResources/StandardMacros.FlipFlop`
      (:`A`
        (bind (_direction _frightened) (`Timeline|Timeline_2` :!label _label_3)
          (:`Update`
            (`SkeletalMeshComponent.SetMorphTarget` (`self.Head`) "disgust" _frightened true))))
      (:`B`
        (goto _label_3 :!via `ReverseFromEnd`)))))

(event `Key|Four`
  (params (Key :type "Key Structure"))
  (:`Pressed`
    (`/Engine/EditorBlueprintResources/StandardMacros.FlipFlop`
      (:`A`
        (bind (_direction _frightened) (`Timeline|Timeline_3` :!label _label_4)
          (:`Update`
            (`SkeletalMeshComponent.SetMorphTarget` (`self.Head`) "sad" _frightened true))))
      (:`B`
        (goto _label_4 :!via `ReverseFromEnd`)))))

(event `Key|Five`
  (params (Key :type "Key Structure"))
  (:`Pressed`
    (`/Engine/EditorBlueprintResources/StandardMacros.FlipFlop`
      (:`A`
        (bind (_direction _frightened) (`Timeline|Timeline_5` :!label _label_5)
          (:`Update`
            (`SkeletalMeshComponent.SetMorphTarget` (`self.Head`) "anger" _frightened true))))
      (:`B`
        (goto _label_5 :!via `ReverseFromEnd`)))))

(event `Key|Six`
  (params (Key :type "Key Structure"))
  (:`Pressed`
    (`/Engine/EditorBlueprintResources/StandardMacros.FlipFlop`
      (:`A`
        (bind (_direction _frightened) (`Timeline|Timeline_6` :!label _label_6)
          (:`Update`
            (`SkeletalMeshComponent.SetMorphTarget` (`self.Head`) "happy" _frightened true))))
      (:`B`
        (goto _label_6 :!via `ReverseFromEnd`)))))

(fn `ARKit_Setup`
  (bind _asarkit (cast `/Game/_Pilivtuber/Moonshine/Skeleton/1030Skeleton/Body/ARKit` (`SkeletalMeshComponent.GetAnimInstance` (`self.Head`))))
  (set `/Game/_Pilivtuber/Moonshine/Skeleton/1030Skeleton/Body/ARKit.LLink Face Subj` (`self.LLink Face Subj`) _asarkit)
  (set `/Game/_Pilivtuber/Moonshine/Skeleton/1030Skeleton/Body/ARKit.LLink Face Head` (`self.LLink Face Head`) _asarkit))

(fn `UserConstructionScript`)