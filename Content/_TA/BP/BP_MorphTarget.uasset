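; BP_MorphTarget plays six facial expression morph targets on a skeletal mesh from numpad keys 1 to 6.
; Each key restarts its own timeline, whose float track drives that expression's morph weight on every update.
; All timelines are read through a track named Frightened, whatever the expression.
; An unconnected alternative using one shared All timeline and a MorphTargetName variable remains in the graph but never runs.
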(event `Key|NumPadOne`
  (params (Key :type "Key Structure"))
  (:`Pressed`
    (bind (_direction _frightened) (`Timeline|frightened` :!via `PlayFromStart`)
      (:`Update`
        (`SkeletalMeshComponent.SetMorphTarget` (`self.SkeletalMesh`) "frightened" _frightened true)))))

(event `Key|NumPadTwo`
  (params (Key :type "Key Structure"))
  (:`Pressed`
    (bind (_direction _frightened) (`Timeline|surprised` :!via `PlayFromStart`)
      (:`Update`
        (`SkeletalMeshComponent.SetMorphTarget` (`self.SkeletalMesh`) "surprised" _frightened true)))))

(event `Key|NumPadThree`
  (params (Key :type "Key Structure"))
  (:`Pressed`
    (bind (_direction _frightened) (`Timeline|disgust` :!via `PlayFromStart`)
      (:`Update`
        (`SkeletalMeshComponent.SetMorphTarget` (`self.SkeletalMesh`) "disgust" _frightened true)))))

(event `Key|NumPadFour`
  (params (Key :type "Key Structure"))
  (:`Pressed`
    (bind (_direction _frightened) (`Timeline|sad` :!via `PlayFromStart`)
      (:`Update`
        (`SkeletalMeshComponent.SetMorphTarget` (`self.SkeletalMesh`) "sad" _frightened true)))))

(event `Key|NumPadFive`
  (params (Key :type "Key Structure"))
  (:`Pressed`
    (bind (_direction _frightened) (`Timeline|anger` :!via `PlayFromStart`)
      (:`Update`
        (`SkeletalMeshComponent.SetMorphTarget` (`self.SkeletalMesh`) "anger" _frightened true)))))

(event `Key|NumPadSix`
  (params (Key :type "Key Structure"))
  (:`Pressed`
    (bind (_direction _frightened) (`Timeline|happy` :!via `PlayFromStart`)
      (:`Update`
        (`SkeletalMeshComponent.SetMorphTarget` (`self.SkeletalMesh`) "happy" _frightened true)))))

(fn `UserConstructionScript`)